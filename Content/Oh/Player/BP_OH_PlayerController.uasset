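; Player controller that provides text chat, push-to-talk voice chat and narrated tutorials for the house, farm, town, shop, bank and clothing areas.
; BeginPlay plays first-visit narration, creates the chat widget and registers the voice talker after a delay.
; Chat messages route through the game mode to everyone.
; Tick rebinds OhQuestUI dialogue events, which advance narration through FlipFlops and boolean stage flags and stop final clips on completion.
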(event `CustomEvent_0`
  (if (`KismetStringLibrary.EqualEqual_StrStr` (`KismetSystemLibrary.GetDisplayName` (`OH_QuestUI.curDialog` (`self.oh_QuestUI`))) "IntroDialogue")
    (`KismetSystemLibrary.PrintString` "2")))

(event `ServerSendMessages`
  (params (Sender :type String) (Message :type String))
  (bind _asbp_hello_future_game_mode (cast `/Game/BP_HelloFutureGameMode` (`GameplayStatics.GetGameMode`)))
  (`/Game/BP_HelloFutureGameMode.SendMessageToEveryone` _asbp_hello_future_game_mode Sender Message))

(event `CreateChatWidget`
  (bind _returnvalue (`|CreateWidget` "/Game/Minsu/Chat/WBP_RealChat.WBP_RealChat_C"))
  (bind _output_get (set `self.Chat` _returnvalue))
  (`UserWidget.AddToViewport` _output_get 0))

(event `AddMessageToChat`
  (params (Sender :type String) (Message :type String))
  (`/Game/Minsu/Chat/WBP_RealChat.AddMessageOntoMessageList` (`self.Chat`) Sender Message))

(event `Key|Zero`
  (params (Key :type "Key Structure"))
  ;[1 1 1] Voice Chat
  (:`Pressed`
    (`AdvancedVoiceLibrary.StartNetworkedVoice` 0))
  (:`Released`
    (`AdvancedVoiceLibrary.StopNetworkedVoice` 0)))

(event `ShowChat`
  (params (Focused :type Boolean))
  (`/Game/Minsu/Chat/WBP_RealChat.Set Focus On Chat` (`self.Chat`) Focused)
  (if Focused
    (`WidgetBlueprintLibrary.SetInputMode_GameAndUIEx` self (`self.Chat`))
    (else
      (`WidgetBlueprintLibrary.SetInputMode_GameOnly` self))))

(event `Key|Enter`
  (params (Key :type "Key Structure"))
  (:`Pressed`
    (`self.ShowChat` true)))

(event `self.ReceiveBeginPlay`
  (`|ExecutionSequence`
    (:`then_0`
      (if (== (`self.isPlaying`) true)
        (bind _returnvalue (`GameplayStatics.SpawnSound2D` "/Game/Oh/Tutorial/Intro_tutorial1.Intro_tutorial1" 1.0 1.0 0.0 null))
        (set `self.Intro_TutorialSound1` _returnvalue)
        (set `self.Tutorial2` true)))
    (:`then_1`
      (if (== (`self.isfirstFarm`) true)
        (bind _returnvalue_2 (`GameplayStatics.SpawnSound2D` "/Game/Oh/Tutorial/Farm_Tutorial1.Farm_Tutorial1" 1.0 1.0 0.0 null))
        (set `self.Farm_TutorialSound1` _returnvalue_2)
        (set `self.farmtutorial2` true)))
    (:`then_2`
      (if (== (`self.isfirstMainMap`) true)
        (bind _returnvalue_3 (`GameplayStatics.SpawnSound2D` "/Game/Oh/Tutorial/TownTutorial1.TownTutorial1" 1.0 1.0 0.0 null))
        (set `self.Town_TutorialSoun1` _returnvalue_3)
        (set `self.Towntutorial1` true)))
    (:`then_3`
      (if (== (`self.isfirstShop`) true)
        (bind _returnvalue_4 (`GameplayStatics.SpawnSound2D` "/Game/Oh/Tutorial/ShopTutorial1_Cue.ShopTutorial1_Cue" 1.0 1.0 0.0 null))
        (set `self.Shop_TutorialSound1` _returnvalue_4)
        (set `self.Shoptutorial1` true)))
    (:`then_4`
      (if (== (`self.isfirstBank`) true)
        (bind _returnvalue_5 (`GameplayStatics.SpawnSound2D` "/Game/Oh/Tutorial/Bank_Tutorial1_Cue.Bank_Tutorial1_Cue" 1.0 1.0 0.0 null))
        (set `self.Bank_TutorialSound1` _returnvalue_5)
        (set `self.Banktutorial1` true)))
    (:`then_5`
      (if (== (`self.isfirstclothing`) true)
        (bind _returnvalue_6 (`GameplayStatics.SpawnSound2D` "/Game/Oh/Tutorial/Clothing_Tutorial1_Cue.Clothing_Tutorial1_Cue" 1.0 1.0 0.0 null))
        (set `self.Clothing_TutorialSound1` _returnvalue_6)
        (set `self.Clothingtutorial1` true)))
    (:`then_6`
      (`self.CreateChatWidget`))
    (:`then_7`
      (`KismetSystemLibrary.Delay` 3.0)
      (`AdvancedVoiceLibrary.RegisterRemoteTalker` (`AdvancedSessionsLibrary.GetUniqueNetID` self)))))

(event `self.ReceiveTick`
  (params (DeltaSeconds :type "Float (single-precision)"))
  (bind _oh_questui (`self.oh_QuestUI`))
  (`/Engine/EditorBlueprintResources/StandardMacros.IsValid` _oh_questui
    (:`Is Valid`
      (add `OH_QuestUI.OnNextDialogueStart` _oh_questui (delegate `OnNextDialogueStart_Event_0`))
      (add `OH_QuestUI.OnDialogueCompleted` _oh_questui (delegate `OnDialogueCompleted_Event_0`)))))

(event `OnNextDialogueStart_Event_0`
  (bind _oh_questui (`self.oh_QuestUI`))
  (bind _farm_tutorialsound1 (`self.Farm_TutorialSound1`))
  (bind _farm_tutorialsound2 (`self.Farm_TutorialSound2`))
  (bind _bank_tutorialsound1 (`self.Bank_TutorialSound1`))
  (bind _oh_questui_2 (`self.oh_QuestUI`))
  (bind _oh_questui_3 (`self.oh_QuestUI`))
  (bind _oh_questui_4 (`self.oh_QuestUI`))
  (bind _oh_questui_5 (`self.oh_QuestUI`))
  (bind _oh_questui_6 (`self.oh_QuestUI`))
  (bind _bank_tutorialsound2 (`self.Bank_TutorialSound2`))
  (bind _bank_tutorialsound3 (`self.Bank_TutorialSound3`))
  (bind _intro_tutorialsound1 (`self.Intro_TutorialSound1`))
  (bind _oh_questui_7 (`self.oh_QuestUI`))
  (bind _oh_questui_8 (`self.oh_QuestUI`))
  (bind _oh_questui_9 (`self.oh_QuestUI`))
  (bind _town_tutorialsoun1 (`self.Town_TutorialSoun1`))
  (bind _town_tutorialsoun2 (`self.Town_TutorialSoun2`))
  (bind _oh_questui_10 (`self.oh_QuestUI`))
  (bind _oh_questui_11 (`self.oh_QuestUI`))
  (bind _oh_questui_12 (`self.oh_QuestUI`))
  (bind _town_tutorialsoun3 (`self.Town_TutorialSoun3`))
  (bind _oh_questui_13 (`self.oh_QuestUI`))
  (bind _shop_tutorialsound1 (`self.Shop_TutorialSound1`))
  (bind _shop_tutorialsound2 (`self.Shop_TutorialSound2`))
  (bind _clothing_tutorialsound1 (`self.Clothing_TutorialSound1`))
  (bind _clothing_tutorialsound2 (`self.Clothing_TutorialSound2`))
  ;[1 1 1] 튜토리얼 다음 대화 시작할 때 다음 소리 나기
  (`|ExecutionSequence`
    (:`then_1`
      ;[1 1 1] House
      (`/Engine/EditorBlueprintResources/StandardMacros.FlipFlop`
        (:`A`
          (if (== (`self.Tutorial2`) true)
            (`/Engine/EditorBlueprintResources/StandardMacros.IsValid` _intro_tutorialsound1
              (:`Is Valid`
                (`AudioComponent.Stop` _intro_tutorialsound1)
                (`/Engine/EditorBlueprintResources/StandardMacros.IsValid` _oh_questui_3
                  (:`Is Valid`
                    (set `OH_QuestUI.finish` true _oh_questui_3)
                    (bind _returnvalue (`GameplayStatics.SpawnSound2D` "/Game/Oh/Tutorial/Intro_Tutorial2.Intro_Tutorial2" 1.0 1.0 0.0 null))
                    (set `self.Intro_TutorialSound2` _returnvalue)
                    (set `OH_QuestUI.finish` false _oh_questui_3)
                    (set `self.Tutorial2` false)
                    (set `self.Tutorial3` true)))))))
        (:`B`
          (if (== (`self.Tutorial3`) true)
            (`/Engine/EditorBlueprintResources/StandardMacros.IsValid` (`self.Intro_TutorialSound2`)
              (:`Is Valid`
                (`ActorComponent.K2_DestroyComponent` (`self.Intro_TutorialSound2`))
                (set `self.Tutorial3` false)))))))
    (:`then_2`
      ;[1 1 1] Farm
      (`/Engine/EditorBlueprintResources/StandardMacros.FlipFlop`
        (:`A`
          (if (== (`self.farmtutorial2`) true)
            (`/Engine/EditorBlueprintResources/StandardMacros.IsValid` _farm_tutorialsound1
              (:`Is Valid`
                (`ActorComponent.K2_DestroyComponent` _farm_tutorialsound1)
                (set `OH_QuestUI.finish` true _oh_questui)
                (bind _returnvalue_2 (`GameplayStatics.SpawnSound2D` "/Game/Oh/Tutorial/FarmTutorial2.FarmTutorial2" 1.0 1.0 0.0 null))
                (set `self.Farm_TutorialSound2` _returnvalue_2)
                (set `OH_QuestUI.finish` false _oh_questui)
                (set `self.farmtutorial2` false)
                (set `self.farmtutorial3` true)))))
        (:`B`
          (if (== (`self.farmtutorial3`) true)
            (`/Engine/EditorBlueprintResources/StandardMacros.IsValid` _farm_tutorialsound2
              (:`Is Valid`
                (`ActorComponent.K2_DestroyComponent` _farm_tutorialsound2)
                (set `OH_QuestUI.finish` true _oh_questui_2)
                (bind _returnvalue_3 (`GameplayStatics.SpawnSound2D` "/Game/Oh/Tutorial/FarmTutorial3.FarmTutorial3" 1.0 1.0 0.0 null))
                (set `OH_QuestUI.finish` false _oh_questui_2)
                (set `self.farmtutorial3` false)
                (set `self.Farm_TutorialSound3` _returnvalue_3)))))))
    (:`then_3`
      ;[1 1 1] Town
      (`/Engine/EditorBlueprintResources/StandardMacros.FlipFlop`
        (:`A`
          (if (== (`self.Towntutorial1`) true)
            (`/Engine/EditorBlueprintResources/StandardMacros.IsValid` _town_tutorialsoun1
              (:`Is Valid`
                (`ActorComponent.K2_DestroyComponent` _town_tutorialsoun1)
                (set `OH_QuestUI.finish` true _oh_questui_7)
                (bind _returnvalue_4 (`GameplayStatics.SpawnSound2D` "/Game/Oh/Tutorial/TownTutorial2.TownTutorial2" 1.0 1.0 0.0 null))
                (set `self.Town_TutorialSoun2` _returnvalue_4)
                (set `OH_QuestUI.finish` false _oh_questui_7)
                (set `self.Towntutorial1` false)
                (set `self.Towntutorial2` true)))))
        (:`B`
          (if (== (`self.Towntutorial2`) true)
            (`/Engine/EditorBlueprintResources/StandardMacros.IsValid` _town_tutorialsoun2
              (:`Is Valid`
                (`ActorComponent.K2_DestroyComponent` _town_tutorialsoun2)
                (set `OH_QuestUI.finish` true _oh_questui_8)
                (bind _returnvalue_5 (`GameplayStatics.SpawnSound2D` "/Game/Oh/Tutorial/TownTutorial3.TownTutorial3" 1.0 1.0 0.0 null))
                (set `self.Town_TutorialSoun3` _returnvalue_5)
                (set `OH_QuestUI.finish` false _oh_questui_8)
                (set `self.Towntutorial2` false)
                (set `self.Towntutorial3` true)))))))
    (:`then_4`
      (`/Engine/EditorBlueprintResources/StandardMacros.FlipFlop`
        (:`A`
          (if (== (`self.Towntutorial3`) true)
            (`/Engine/EditorBlueprintResources/StandardMacros.IsValid` _town_tutorialsoun3
              (:`Is Valid`
                (`ActorComponent.K2_DestroyComponent` _town_tutorialsoun3)
                (set `OH_QuestUI.finish` true _oh_questui_12)
                (bind _returnvalue_6 (`GameplayStatics.SpawnSound2D` "/Game/Oh/Tutorial/TownTutorial4.TownTutorial4" 1.0 1.0 0.0 null))
                (set `self.Town_TutorialSoun4` _returnvalue_6)
                (set `OH_QuestUI.finish` false _oh_questui_12)
                (set `self.Towntutorial3` false)))))))
    (:`then_5`
      ;[1 1 1] Shop
      (`/Engine/EditorBlueprintResources/StandardMacros.FlipFlop`
        (:`A`
          (if (== (`self.Shoptutorial1`) true)
            (`/Engine/EditorBlueprintResources/StandardMacros.IsValid` _shop_tutorialsound1
              (:`Is Valid`
                (`ActorComponent.K2_DestroyComponent` _shop_tutorialsound1)
                (set `OH_QuestUI.finish` true _oh_questui_11)
                (bind _returnvalue_7 (`GameplayStatics.SpawnSound2D` "/Game/Oh/Tutorial/ShopTutorial2_Cue.ShopTutorial2_Cue" 1.0 1.0 0.0 null))
                (set `self.Shop_TutorialSound2` _returnvalue_7)
                (set `OH_QuestUI.finish` false _oh_questui_11)
                (set `self.Shoptutorial1` false)
                (set `self.Shoptutorial2` true)))))
        (:`B`
          (if (== (`self.Shoptutorial2`) true)
            (`/Engine/EditorBlueprintResources/StandardMacros.IsValid` _shop_tutorialsound2
              (:`Is Valid`
                (`ActorComponent.K2_DestroyComponent` _shop_tutorialsound2)
                (set `OH_QuestUI.finish` true _oh_questui_13)
                (bind _returnvalue_8 (`GameplayStatics.SpawnSound2D` "/Game/Oh/Tutorial/ShopTutorial3_Cue.ShopTutorial3_Cue" 1.0 1.0 0.0 null))
                (set `self.Shop_TutorialSound3` _returnvalue_8)
                (set `OH_QuestUI.finish` false _oh_questui_13)
                (set `self.Shoptutorial2` false)))))))
    (:`then_6`
      ;[1 1 1] Bank
      (`/Engine/EditorBlueprintResources/StandardMacros.FlipFlop`
        (:`A`
          (if (== (`self.Banktutorial1`) true)
            (`/Engine/EditorBlueprintResources/StandardMacros.IsValid` _bank_tutorialsound1
              (:`Is Valid`
                (`ActorComponent.K2_DestroyComponent` _bank_tutorialsound1)
                (set `OH_QuestUI.finish` true _oh_questui_4)
                (bind _returnvalue_9 (`GameplayStatics.SpawnSound2D` "/Game/Oh/Tutorial/Bank_Tutorial2_Cue.Bank_Tutorial2_Cue" 1.0 1.0 0.0 null))
                (set `self.Bank_TutorialSound2` _returnvalue_9)
                (set `OH_QuestUI.finish` false _oh_questui_4)
                (set `self.Banktutorial1` false)
                (set `self.Banktutorial2` true)))))
        (:`B`
          (if (== (`self.Banktutorial2`) true)
            (`/Engine/EditorBlueprintResources/StandardMacros.IsValid` _bank_tutorialsound2
              (:`Is Valid`
                (`ActorComponent.K2_DestroyComponent` _bank_tutorialsound2)
                (set `OH_QuestUI.finish` true _oh_questui_5)
                (bind _returnvalue_10 (`GameplayStatics.SpawnSound2D` "/Game/Oh/Tutorial/Bank_Tutorial3.Bank_Tutorial3" 1.0 1.0 0.0 null))
                (set `self.Bank_TutorialSound3` _returnvalue_10)
                (set `OH_QuestUI.finish` false _oh_questui_5)
                (set `self.Banktutorial2` false)
                (set `self.Banktutorial3` true)))))))
    (:`then_7`
      (`/Engine/EditorBlueprintResources/StandardMacros.FlipFlop`
        (:`A`
          (if (== (`self.Banktutorial3`) true)
            (`/Engine/EditorBlueprintResources/StandardMacros.IsValid` _bank_tutorialsound3
              (:`Is Valid`
                (`ActorComponent.K2_DestroyComponent` _bank_tutorialsound3)
                (set `OH_QuestUI.finish` true _oh_questui_9)
                (bind _returnvalue_11 (`GameplayStatics.SpawnSound2D` "/Game/Oh/Tutorial/Bank_Tutorial4_Cue.Bank_Tutorial4_Cue" 1.0 1.0 0.0 null))
                (set `self.Bank_TutorialSound4` _returnvalue_11)
                (set `OH_QuestUI.finish` false _oh_questui_9)
                (set `self.Banktutorial3` false)))))))
    (:`then_8`
      ;[1 1 1] Clothing
      (`/Engine/EditorBlueprintResources/StandardMacros.FlipFlop`
        (:`A`
          (if (== (`self.Clothingtutorial1`) true)
            (`/Engine/EditorBlueprintResources/StandardMacros.IsValid` _clothing_tutorialsound1
              (:`Is Valid`
                (`ActorComponent.K2_DestroyComponent` _clothing_tutorialsound1)
                (set `OH_QuestUI.finish` true _oh_questui_10)
                (bind _returnvalue_12 (`GameplayStatics.SpawnSound2D` "/Game/Oh/Tutorial/33333_Cue.33333_Cue" 1.0 1.0 0.0 null))
                (set `self.Clothing_TutorialSound2` _returnvalue_12)
                (set `OH_QuestUI.finish` false _oh_questui_10)
                (set `self.Clothingtutorial1` false)
                (set `self.Clothingtutorial2` true)))))
        (:`B`
          (if (== (`self.Clothingtutorial2`) true)
            (`/Engine/EditorBlueprintResources/StandardMacros.IsValid` _clothing_tutorialsound2
              (:`Is Valid`
                (`ActorComponent.K2_DestroyComponent` _clothing_tutorialsound2)
                (set `OH_QuestUI.finish` true _oh_questui_6)
                (bind _returnvalue_13 (`GameplayStatics.SpawnSound2D` "/Game/Oh/Tutorial/Clothing_Tutorial3_Cue.Clothing_Tutorial3_Cue" 1.0 1.0 0.0 null))
                (set `self.Clothing_TutorialSound3` _returnvalue_13)
                (set `OH_QuestUI.finish` false _oh_questui_6)
                (set `self.Clothingtutorial2` false)))))))))

(event `OnDialogueCompleted_Event_0`
  (bind _town_tutorialsoun4 (`self.Town_TutorialSoun4`))
  (bind _shop_tutorialsound3 (`self.Shop_TutorialSound3`))
  (bind _bank_tutorialsound4 (`self.Bank_TutorialSound4`))
  (bind _clothing_tutorialsound3 (`self.Clothing_TutorialSound3`))
  (bind _farm_tutorialsound3 (`self.Farm_TutorialSound3`))
  ;[1 1 1] 튜토리얼 대화 완전히 끝나도 소리 끄기
  (`|ExecutionSequence`
    (:`then_1`
      (`/Engine/EditorBlueprintResources/StandardMacros.IsValid` _farm_tutorialsound3
        (:`Is Valid`
          (`ActorComponent.K2_DestroyComponent` _farm_tutorialsound3))))
    (:`then_2`
      (`/Engine/EditorBlueprintResources/StandardMacros.IsValid` _town_tutorialsoun4
        (:`Is Valid`
          (`ActorComponent.K2_DestroyComponent` _town_tutorialsoun4))))
    (:`then_3`
      (`/Engine/EditorBlueprintResources/StandardMacros.IsValid` _shop_tutorialsound3
        (:`Is Valid`
          (`ActorComponent.K2_DestroyComponent` _shop_tutorialsound3))))
    (:`then_4`
      (`/Engine/EditorBlueprintResources/StandardMacros.IsValid` _bank_tutorialsound4
        (:`Is Valid`
          (`ActorComponent.K2_DestroyComponent` _bank_tutorialsound4))))
    (:`then_5`
      (`/Engine/EditorBlueprintResources/StandardMacros.IsValid` _clothing_tutorialsound3
        (:`Is Valid`
          (`ActorComponent.K2_DestroyComponent` _clothing_tutorialsound3))))))

(fn `UserConstructionScript`)