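; Farm tree actor that spawns fruit after a hold-to-shake interaction, with a montage on the player character.
; A gated retriggerable delay triggers the spawn if still held, while a polling timer feeds hold time to WBP_Hold.
; The input triggers and overlap setup that opens the gate are disconnected.
; A note marks logic for deletion, saying YJ_HelloFutrueCharacter now implements it.
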(event `Spawn Actor On Server`
  ;[1 1 1] 삭제 예정(YJ_HelloFutrueCharacter에 구현함)
  (`self.SpawnFruit`))

(event `Play Animation`
  ;[1 1 1] 삭제 예정(YJ_HelloFutrueCharacter에 구현함)
  (set `self.Is Held?` true)
  (`Character.PlayAnimMontage` (`GameplayStatics.GetPlayerCharacter` 0) "/Game/Map/Animation/Shake_Gesture_Montage.Shake_Gesture_Montage" 1.0 "None")
  (`/Engine/EditorBlueprintResources/StandardMacros.Gate` true
    (:`Exit`
      (`|ExecutionSequence`
        (:`then_0`
          (`KismetSystemLibrary.RetriggerableDelay` (`self.MaxHoldTime`))
          (if (`self.Is Held?`)
            (`Widget.RemoveFromParent` (`self.Hold Widget`))
            (`self.Spawn Actor On Server`)))
        (:`then_1`
          (`self.Timer`)
          (`self.Update Timer`))))))

(event `Stop Animation`
  ;[1 1 1] 삭제 예정(YJ_HelloFutrueCharacter에 구현함)
  (set `self.Is Held?` false)
  (`Character.StopAnimMontage` (`GameplayStatics.GetPlayerCharacter` 0) "/Game/Map/Animation/Shake_Gesture_Montage.Shake_Gesture_Montage"))

(event `self.Box.OnComponentBeginOverlap`
  (params (OverlappedComponent :type "PrimitiveComponent Object Reference") (OtherActor :type "Actor Object Reference") (OtherComp :type "PrimitiveComponent Object Reference") (OtherBodyIndex :type Integer) (bFromSweep :type Boolean) (SweepResult :type "HitResult Structure (by ref)"))
  ;[1 1 1] 삭제 예정(YJ_HelloFutrueCharacter에 구현함)
)

(event `Stop Timer`
  ;[1 1 1] 삭제 예정(YJ_HelloFutrueCharacter에 구현함)
  (`KismetSystemLibrary.K2_PauseTimerHandle` (stale `Timer` _returnvalue)))

(event `self.Box.OnComponentEndOverlap`
  (params (OverlappedComponent :type "PrimitiveComponent Object Reference") (OtherActor :type "Actor Object Reference") (OtherComp :type "PrimitiveComponent Object Reference") (OtherBodyIndex :type Integer))
  ;[1 1 1] 삭제 예정(YJ_HelloFutrueCharacter에 구현함)
)

(event `Timer`
  ;[1 1 1] 삭제 예정(YJ_HelloFutrueCharacter에 구현함)
  (bind _returnvalue (`KismetSystemLibrary.K2_SetTimerDelegate` (delegate `Timer`) (`self.MaxHoldTime`))))

(event `Update Timer`
  (bind _hold_widget (`self.Hold Widget`))
  ;[1 1 1] 삭제 예정(YJ_HelloFutrueCharacter에 구현함)
  (if (`self.Is Held?`)
    (set `/Game/Minsu/Farm/BP/WBP_Hold.TimeHeld` (`KismetSystemLibrary.K2_GetTimerElapsedTimeHandle` (stale `Timer` _returnvalue)) _hold_widget)
    (`KismetSystemLibrary.Delay` 0.1)
    (`self.Update Timer`)
    (else
      (`self.Stop Timer`)
      (set `/Game/Minsu/Farm/BP/WBP_Hold.TimeHeld` 0.0 _hold_widget))))

(fn `UserConstructionScript`)