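; BP_WheatSeed is a farm pickup that adds a wheat seed to the player's inventory.
; Overlapping its Box makes a HelloFutureCharacter play a planting montage with input disabled for a second, then plays a pickup sound, grants the seed and destroys the actor.
; That path also notifies each quest in the YJ_HelloFutureCharacter's QuestLog of the collected item.
; Interact2 is a direct alternative that only grants the seed and destroys the actor.
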(event `self.Box.OnComponentBeginOverlap`
  (params (OverlappedComponent :type "PrimitiveComponent Object Reference") (OtherActor :type "Actor Object Reference") (OtherComp :type "PrimitiveComponent Object Reference") (OtherBodyIndex :type Integer) (bFromSweep :type Boolean) (SweepResult :type "HitResult Structure (by ref)"))
  (bind _returnvalue (`GameplayStatics.GetPlayerController` 0))
  (bind _ashello_future_character (cast `HelloFutureCharacter` OtherActor))
  (`Character.PlayAnimMontage` _ashello_future_character "/Game/Map/Animation/Plant2_Montage1.Plant2_Montage1" 1.0 "None")
  (`self.DisableInput` _ashello_future_character _returnvalue)
  (`KismetSystemLibrary.Delay` 1.0)
  (`GameplayStatics.PlaySound2D` "/Game/NewAssets/Game_UI_Bundle/Casual_Game_UI_Sound/Cue/USER_INTERFACE/USER_INTERFACE_Get_Item_02_Cue.USER_INTERFACE_Get_Item_02_Cue" 1.0 1.0 0.0 null null)
  (`self.EnableInput` _ashello_future_character _returnvalue)
  ;[1 1 1] CornItem 아이템 추가
  (`YJ_InventoryComponent.AddItem2` (`HelloFutureCharacter.Inventory` _ashello_future_character) "WheatSeed")
  (`self.K2_DestroyActor`)
  (bind _asyj_hello_future_character (cast `/Game/Map/YJ_HelloFutureCharacter` (`GameplayStatics.GetPlayerCharacter` 0)))
  (for _array_element (`/Game/Oh/RealQuest/QuestLog.Quests` (`/Game/Map/YJ_HelloFutureCharacter.QuestLog` _asyj_hello_future_character))
    (`/Game/Oh/RealQuest/Quests/OH_RealQuest.CollectedItem` _array_element "WheatSeed")))

(event `/Game/Oh/RealQuest/InteractInterface.Interact2`
  (bind _asyj_hello_future_character (cast `/Game/Map/YJ_HelloFutureCharacter` (`GameplayStatics.GetPlayerCharacter` 0)))
  ;[1 1 1] CornItem 아이템 추가
  (`YJ_InventoryComponent.AddItem2` (`HelloFutureCharacter.Inventory` _asyj_hello_future_character) "WheatSeed")
  (`self.K2_DestroyActor`))

(fn `UserConstructionScript`)