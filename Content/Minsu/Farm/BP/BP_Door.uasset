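; BP_Door is a door actor that shows a door UI widget when a HelloFutureCharacter enters either of its two trigger spheres.
; Each sphere creates its own widget for player controller 0, passing the door reference, then removes it on exit and restores game-only input.
; Remote-only authority checks are disconnected, so any overlapping character of that class triggers this logic.
; An author note marks it for deletion, as YJ_HelloFutureCharacter implements it.
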(event `self.ReceiveBeginPlay`
  ;[1 1 1] 삭제예정 (YJ_HelloFutureCharacter에 구현함)
)

(event `self.Sphere.OnComponentBeginOverlap`
  (params (OverlappedComponent :type "PrimitiveComponent Object Reference") (OtherActor :type "Actor Object Reference") (OtherComp :type "PrimitiveComponent Object Reference") (OtherBodyIndex :type Integer) (bFromSweep :type Boolean) (SweepResult :type "HitResult Structure (by ref)"))
  ;[1 1 1] 삭제예정 (YJ_HelloFutureCharacter에 구현함)
  (cast `HelloFutureCharacter` OtherActor)
  (bind _returnvalue (`|CreateWidget` "/Game/Minsu/NewWBP_Door01.NewWBP_Door01_C" (`GameplayStatics.GetPlayerController` 0) self))
  (`UserWidget.AddToViewport` _returnvalue 0))

(event `self.Sphere.OnComponentEndOverlap`
  (params (OverlappedComponent :type "PrimitiveComponent Object Reference") (OtherActor :type "Actor Object Reference") (OtherComp :type "PrimitiveComponent Object Reference") (OtherBodyIndex :type Integer))
  ;[1 1 1] 삭제예정 (YJ_HelloFutureCharacter에 구현함)
  (cast `HelloFutureCharacter` OtherActor)
  (`/Engine/EditorBlueprintResources/StandardMacros.IsValid` (stale `self.Sphere.OnComponentBeginOverlap` _returnvalue)
    (:`Is Valid`
      (`Widget.RemoveFromParent` (stale `self.Sphere.OnComponentBeginOverlap` _returnvalue))
      (`WidgetBlueprintLibrary.SetInputMode_GameOnly` (`GameplayStatics.GetPlayerController` 0)))))

(event `self.Sphere1.OnComponentBeginOverlap`
  (params (OverlappedComponent :type "PrimitiveComponent Object Reference") (OtherActor :type "Actor Object Reference") (OtherComp :type "PrimitiveComponent Object Reference") (OtherBodyIndex :type Integer) (bFromSweep :type Boolean) (SweepResult :type "HitResult Structure (by ref)"))
  ;[1 1 1] 삭제예정 (YJ_HelloFutureCharacter에 구현함)
  (cast `HelloFutureCharacter` OtherActor)
  (bind _returnvalue (`|CreateWidget` "/Game/Minsu/NewWBP_Door01.NewWBP_Door01_C" (`GameplayStatics.GetPlayerController` 0) self))
  (`UserWidget.AddToViewport` _returnvalue 0))

(event `self.Sphere1.OnComponentEndOverlap`
  (params (OverlappedComponent :type "PrimitiveComponent Object Reference") (OtherActor :type "Actor Object Reference") (OtherComp :type "PrimitiveComponent Object Reference") (OtherBodyIndex :type Integer))
  ;[1 1 1] 삭제예정 (YJ_HelloFutureCharacter에 구현함)
  (cast `HelloFutureCharacter` OtherActor)
  (`/Engine/EditorBlueprintResources/StandardMacros.IsValid` (stale `self.Sphere1.OnComponentBeginOverlap` _returnvalue)
    (:`Is Valid`
      (`Widget.RemoveFromParent` (stale `self.Sphere1.OnComponentBeginOverlap` _returnvalue))
      (`WidgetBlueprintLibrary.SetInputMode_GameOnly` (`GameplayStatics.GetPlayerController` 0)))))

(fn `UserConstructionScript`)