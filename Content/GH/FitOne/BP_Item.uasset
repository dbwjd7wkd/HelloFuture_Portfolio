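; BP_Item is a clickable clothing item that sends its mesh and materials to the FitOneController to change the worn outfit.
; On BeginPlay it flags multi-material meshes and builds a hidden outline copy of its skeletal mesh using a highlight material.
; Box cursor events toggle that outline on hover, and a click calls the single- or multi-material change function with category and object name.
; Older toggle and double-click removal logic remains unwired.
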(event `SetOuterSkeletalMesh`
  (bind _outlineskeletal (`self.outlineSkeletal`))
  (`SkinnedMeshComponent.SetSkinnedAssetAndUpdate` _outlineskeletal (`SkinnedMeshComponent.SkeletalMesh` (`self.SkeletalMesh`)) true)
  (for (_ _array_index) (`MeshComponent.GetMaterials` _outlineskeletal)
    (`PrimitiveComponent.SetMaterial` (`self.outlineSkeletal`) _array_index "/Game/GH/FitOne/Clicked_M_Inst.Clicked_M_Inst")
    (`SceneComponent.SetVisibility` (`self.outlineSkeletal`) false false)))

(event `self.ReceiveBeginPlay`
  (bind _outlineskeletal (`self.outlineSkeletal`))
  (`|ExecutionSequence`
    (:`then_0`
      (bind _asfit_one_controller (cast `/Game/GH/FitOne/FitOneController` (`GameplayStatics.GetPlayerController` 0)))
      (set `self.FitOneController` _asfit_one_controller)
      ;[1 1 1] 클릭한 아이템이 여러개의 머터리얼인지 확인
      (if (> (`KismetArrayLibrary.Array_Length` (`MeshComponent.GetMaterials` (`self.SkeletalMesh`))) 1)
        (set `self.isMulti` true)))
    (:`then_1`
      (`SkinnedMeshComponent.SetSkinnedAssetAndUpdate` _outlineskeletal (`SkinnedMeshComponent.SkeletalMesh` (`self.SkeletalMesh`)) true)
      (for (_ _array_index) (`MeshComponent.GetMaterials` _outlineskeletal)
        (`PrimitiveComponent.SetMaterial` (`self.outlineSkeletal`) _array_index "/Game/GH/FitOne/Clicked_M_Inst.Clicked_M_Inst")
        (`SceneComponent.SetVisibility` (`self.outlineSkeletal`) false false)))))

(event `self.Box.OnBeginCursorOver`
  (params (TouchedComponent :type "PrimitiveComponent Object Reference"))
  ;[1 1 1] 호버 시 하이라이팅
  (`SceneComponent.SetVisibility` (`self.outlineSkeletal`) true false))

(event `self.Box.OnEndCursorOver`
  (params (TouchedComponent :type "PrimitiveComponent Object Reference"))
  ;[1 1 1] 호버 시 하이라이팅
  (`SceneComponent.SetVisibility` (`self.outlineSkeletal`) false false))

(event `self.Box.OnClicked`
  (params (TouchedComponent :type "PrimitiveComponent Object Reference") (ButtonPressed :type "Key Structure"))
  (bind _skeletalmesh (`self.SkeletalMesh`))
  (bind _clothescategory (`self.ClothesCategory`))
  (bind _fitonecontroller (`self.FitOneController`))
  (bind _returnvalue (`MeshComponent.GetMaterials` _skeletalmesh))
  (bind _returnvalue_2 (`KismetSystemLibrary.GetObjectName` self))
  (bind _skeletalmesh_2 (`SkinnedMeshComponent.SkeletalMesh` _skeletalmesh))
  (`GameplayStatics.GetActorOfClass` "/Game/GH/FitOne/BP_PrettyBoneActor.BP_PrettyBoneActor_C")
  (if (`self.isMulti`)
    (`/Game/GH/FitOne/FitOneController.CTR_FitOneChangeMultiMat` _fitonecontroller _clothescategory _returnvalue _skeletalmesh_2 false _returnvalue_2)
    (else
      (`/Game/GH/FitOne/FitOneController.CTR_FitOne_Change` _fitonecontroller _clothescategory (`|GetArrayItem` _returnvalue) _skeletalmesh_2 true _returnvalue_2))))

(fn `UserConstructionScript`)